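; Behavior tree task that chooses the next patrol waypoint for an AI-controlled NPC.
; On execute it casts the controlled pawn to read its patrol points array, then writes the point at the blackboard Index to the Waypoint key as an object.
; It then increments Index modulo the array length, so the route loops, and finishes successfully.
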(event EventReceiveExecuteAI
  (params (OwnerController :type AI%20Controller%20Object%20Reference) (ControlledPawn :type Pawn%20Object%20Reference))
  (CallFunction|GetPatrolPoints ControlledPawn)
  (bind _index (CallFunction|SetPatrolPoints))
  (CallFunction|CycleIndex _index)
  (AI|BehaviorTree|FinishExecute true))

(fn GetPatrolPoints
  (params (Object :type Object%20Object%20Reference))
  (Utilities|Casting|CastTo Object)
  (Variables|Default|SetPatrol%20Points (Variables|Default|GetPatrol%20Points)))

(fn SetPatrolPoints
  (bind _index (Variables|Default|GetIndex))
  (bind _returnvalue (Class|BTFunctionLibrary|GetBlackboardValueasInt _index))
  (Class|BTFunctionLibrary|SetBlackboardValueasObject (Variables|Default|GetWaypoint) (Utilities|Array|Get(acopy) (Variables|Default|GetPatrol%20Points) _returnvalue))
  (return _returnvalue))

(fn CycleIndex
  (params (Index :type Integer))
  (Class|BTFunctionLibrary|SetBlackboardValueasInt (Variables|Default|GetIndex) (Math|Integer|%(Integer) (+ Index 1) (Utilities|Array|Length (Variables|Default|GetPatrol%20Points)))))